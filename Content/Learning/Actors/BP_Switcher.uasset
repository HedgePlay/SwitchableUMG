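; BP_Switcher is an interactable switch actor that shows a widget while something overlaps its sphere.
; On BeginPlay it hides the widget and caches every actor tagged "SwitchingActors".
; Its Switch event loops over that cached list, calling the OnPressed dispatcher once per entry.
; IsSwitchOn exposes the IsOn state, which none of these graphs changes.
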(event OnComponentBeginOverlap(Sphere)
  (params (OverlappedComponent :type Primitive%20Component%20Object%20Reference) (OtherActor :type Actor%20Object%20Reference) (OtherComp :type Primitive%20Component%20Object%20Reference) (OtherBodyIndex :type Integer) (bFromSweep :type Boolean) (SweepResult :type Hit%20Result%20Structure%20%28by%20ref%29))
  (Rendering|SetVisibility (Variables|Default|GetWidget) true false))

(event OnComponentEndOverlap(Sphere)
  (params (OverlappedComponent :type Primitive%20Component%20Object%20Reference) (OtherActor :type Actor%20Object%20Reference) (OtherComp :type Primitive%20Component%20Object%20Reference) (OtherBodyIndex :type Integer))
  (Rendering|SetVisibility (Variables|Default|GetWidget) false false))

(event EventBeginPlay
  (Rendering|SetVisibility (Variables|Default|GetWidget) false false)
  (bind _outactors (Actor|GetAllActorswithTag "SwitchingActors"))
  (Variables|Default|SetActorsToSwitch _outactors))

(event EventSwitch
  (for _array_element (Variables|Default|GetActorsToSwitch)
    (Default|CallOnPressed)))

(fn ConstructionScript)

(fn IsSwitchon
  (return (Variables|Default|GetisOn)))