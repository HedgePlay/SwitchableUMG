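; BP_Switcher1 is a proximity-activated switch actor with a widget interface and an IsOn state query.
; Overlapping its sphere shows the widget and mouse cursor in Game-and-UI input; leaving restores game-only input.
; BeginPlay hides the widget and fills ActorsToSwitch from actors tagged "SwitchingActors", assigning a single-element array each iteration.
; Switch calls OnPressed once per stored entry; the widget's click handler is empty.
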(event OnComponentBeginOverlap(Sphere)
  (params (OverlappedComponent :type Primitive%20Component%20Object%20Reference) (OtherActor :type Actor%20Object%20Reference) (OtherComp :type Primitive%20Component%20Object%20Reference) (OtherBodyIndex :type Integer) (bFromSweep :type Boolean) (SweepResult :type Hit%20Result%20Structure%20%28by%20ref%29))
  (bind _returnvalue (Game|GetPlayerController 0))
  (bind _widget (Variables|Default|GetWidget))
  (Rendering|SetVisibility _widget true false)
  (Variables|/Script/Engine.PlayerController|SetbShowMouseCursor _returnvalue true)
  (Input|SetInputModeGameandUI _returnvalue (UserInterface|GetWidget _widget) "LockAlways" true false))

(event OnComponentEndOverlap(Sphere)
  (params (OverlappedComponent :type Primitive%20Component%20Object%20Reference) (OtherActor :type Actor%20Object%20Reference) (OtherComp :type Primitive%20Component%20Object%20Reference) (OtherBodyIndex :type Integer))
  (bind _returnvalue (Game|GetPlayerController 0))
  (Rendering|SetVisibility (Variables|Default|GetWidget) false false)
  (Variables|/Script/Engine.PlayerController|SetbShowMouseCursor _returnvalue false)
  (Input|SetInputModeGameOnly _returnvalue false))

(event OnClicked(Widget)
  (params (TouchedComponent :type Primitive%20Component%20Object%20Reference) (ButtonPressed :type Key%20Structure :default "None")))

(event EventBeginPlay
  (Rendering|SetVisibility (Variables|Default|GetWidget) false false)
  (bind _outactors (Actor|GetAllActorswithTag "SwitchingActors"))
  (for _array_element _outactors
    (Variables|Default|SetActorsToSwitch (Utilities|Array|MakeArray _array_element))))

(event EventSwitch
  (for _array_element (Variables|Default|GetActorsToSwitch)
    (Default|CallOnPressed)))

(fn ConstructionScript)

(fn IsSwitchon
  (return (Variables|Default|GetisOn)))